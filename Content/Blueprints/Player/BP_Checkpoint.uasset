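; BP_Checkpoint is a player checkpoint that sets the spawn location and can calm the enemies in its room.
; When the player pawn overlaps its Box, it passes itself to BP_QoriGameMode's UpdateSpawnLocation.
; Its ReloadRoom function, not called within this Blueprint, loops over EnemiesInRoom and sets each AIC_Enemy_Base controller to passive.
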(event `self.Box.OnComponentBeginOverlap`
  (params (OverlappedComponent :type "PrimitiveComponent Object Reference") (OtherActor :type "Actor Object Reference") (OtherComp :type "PrimitiveComponent Object Reference") (OtherBodyIndex :type Integer) (bFromSweep :type Boolean) (SweepResult :type "HitResult Structure (by ref)"))
  (if (== OtherActor (`GameplayStatics.GetPlayerPawn` 0))
    (bind _asbp_qori_game_mode (cast `/Game/Blueprints/BP_QoriGameMode` (`GameplayStatics.GetGameMode`)))
    (`/Game/Blueprints/BP_QoriGameMode.UpdateSpawnLocation` _asbp_qori_game_mode self)))

(fn `ReloadRoom`
  (for _array_element (`self.EnemiesInRoom`)
    (bind _asaic_enemy_base (cast `/Game/Blueprints/Enemy/AI/AIC_Enemy_Base` (`AIBlueprintHelperLibrary.GetAIController` _array_element)))
    (`/Game/Blueprints/Enemy/AI/AIC_Enemy_Base.SetStateAsPassive` _asaic_enemy_base)))

(fn `UserConstructionScript`)