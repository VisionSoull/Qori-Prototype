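; BP_StatuesManager runs a statue rotation puzzle, tracking a set of statues and the objects to activate once it is solved.
; On BeginPlay it registers itself with each statue and prunes invalid statues and entries lacking BPI_Activable.
; CheckCorrectRotations completes the puzzle when every statue is correctly rotated, locking the statues and messaging each activable.
; Helpers spawn, add and remove statues, and the construction script clears invalid array slots.
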(event `self.ReceiveBeginPlay`
  (`self.VerifyStatues`)
  (`self.VerifyValidActivables`))

(fn `AddStatueToArray`
  (params (Statue :type "/Game/Blueprints/Statues/BP_Statue Object Reference"))
  (`KismetArrayLibrary.Array_AddUnique` (`self.AllStatues`) Statue)
  (`/Game/Blueprints/Statues/BP_Statue.SetStatuesManager` Statue self))

(fn `CeateNewStatue`
  (bind _returnvalue (`|SpawnActorFromClass` (`self.StatueClass`) (`self.GetTransform`) "Undefined" "MultiplyWithRoot" null null))
  (`self.AddStatueToArray` _returnvalue))

(fn `CheckCorrectRotations`
  (for _array_element (`self.AllStatues`)
    (if (`/Game/Blueprints/Statues/BP_Statue.CorrectRotation` _array_element)
      (set `self.bStatuesComplete` true)
      (else
        (set `self.bStatuesComplete` false)
        (break))))
  (if (`self.bStatuesComplete`)
    (`self.CompletePuzzle`)))

(fn `CompletePuzzle`
  (for _array_element (`self.AllStatues`)
    (`/Game/Blueprints/Statues/BP_Statue.SetNotInteractable` _array_element))
  (for _array_element_2 (`self.Activables`)
    (message `/Game/Blueprints/Interfaces/BPI_Activable.Activate` _array_element_2)))

(fn `RemoveStatueFromArray`
  (params (Statue :type "/Game/Blueprints/Statues/BP_Statue Object Reference"))
  (`KismetArrayLibrary.Array_RemoveItem` (`self.AllStatues`) Statue)
  (`self.VerifyStatues`))

(fn `UserConstructionScript`
  (for (_array_element _array_index) (`self.AllStatues`)
    (`/Engine/EditorBlueprintResources/StandardMacros.IsValid` _array_element
      (:`Is Not Valid`
        (`KismetArrayLibrary.Array_Set` (`self.AllStatues`) _array_index)
        (if (not (`KismetArrayLibrary.Array_IsEmpty` (`self.Activables`)))
          (for (_array_element_2 _array_index_2) (`self.Activables`)
            (`/Engine/EditorBlueprintResources/StandardMacros.IsValid` _array_element_2
              (:`Is Valid`
                (cast `/Game/Blueprints/Interfaces/BPI_Activable` _array_element_2
                  (:`CastFailed`
                    (`KismetArrayLibrary.Array_Set` (`self.Activables`) _array_index_2)))))))))))

(fn `VerifyStatues`
  ;[1 1 1] Verify if there are empty indexes in the array and remove them
  (for (_array_element _array_index) (`self.AllStatues`)
    (`/Engine/EditorBlueprintResources/StandardMacros.IsValid` _array_element
      (:`Is Valid`
        (`/Game/Blueprints/Statues/BP_Statue.SetStatuesManager` _array_element self))
      (:`Is Not Valid`
        (`KismetArrayLibrary.Array_Remove` (`self.AllStatues`) _array_index)))))

(fn `VerifyValidActivables`
  (for (_array_element _array_index) (`self.Activables`)
    (cast `/Game/Blueprints/Interfaces/BPI_Activable` _array_element
      (:`CastFailed`
        (`KismetArrayLibrary.Array_Remove` (`self.Activables`) _array_index)))))