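; BP_Torch is an environment torch with a point light and a torch effect, which can start lit or unlit.
; The construction script applies the color, radius and intensity variables to the light and sets light and effect visibility from IsLitUp, including the effect's children.
; The Activate event calls VisibleNotVisible, which toggles only the point light's visibility, leaving the effect and IsLitUp unchanged.
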(event `/Game/Blueprints/Interfaces/BPI_Activable.Activate`
  (`self.Visible/NotVisible`))

(fn `UserConstructionScript`
  (`LightComponent.SetLightColor` (`self.PointLight`) (`self.LightColor`) true)
  (`LocalLightComponent.SetAttenuationRadius` (`self.PointLight`) (`self.Radius`))
  (`LightComponent.SetIntensity` (`self.PointLight`) (`self.Intensity`))
  (`SceneComponent.SetVisibility` (`self.PointLight`) (`self.bIsLitUp`) false)
  (`SceneComponent.SetVisibility` (`self.FXS_Torches`) (`self.bIsLitUp`) true))

(fn `Visible/NotVisible`
  (`SceneComponent.ToggleVisibility` (`self.PointLight`) false))