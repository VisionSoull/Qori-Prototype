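; Base enemy character that handles health, weapon wielding, patrol route and speed helpers, and death, leaving attack logic to children.
; Construction links BPCDamageSystem's death event and creates two dynamic materials; BeginPlay spawns the socketed weapon and health bar widget.
; Damage, healing and health queries forward to the damage component.
; Death detaches and decays the weapon, ragdolls the mesh, then fades both materials on a timeline before destroying the actor.
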(event `self.ReceiveBeginPlay`
  (`self.Wield Weapon`)
  ;[0 0.1277 0.1719] Create Health Bar Widget
  (bind _returnvalue (`|CreateWidget` "/Game/UI/W_HealthBar.W_HealthBar_C" null self))
  (`WidgetComponent.SetWidget` (`self.HealthBar`) _returnvalue))

(event `Attack`
  ;[0.1892 0.05327 0.4167] Attack Event to be used by children. Only verifies if it has a weapon
  (`self.Weapon`
    (:`then`
      (`KismetSystemLibrary.PrintString` ""))
    (:`else`)))

(event `Wield Weapon`
  ;[0.1875 0.1515 0] Wield Weapon if "Weapon" is valid
  (bind _weapon (`self.Weapon`)
    (:`then`
      (bind _returnvalue (`|SpawnActorFromClass` _weapon (`self.GetTransform`) "Undefined" "MultiplyWithRoot" null null))
      (bind _output_get (set `self.WeaponObject` _returnvalue))
      (`/Game/Blueprints/Weapons/BP_Weapon.SetupWeapon` _output_get self (`self.AttackDamageAmount`))
      (`self.K2_AttachToComponent` _output_get (`self.Mesh`) "hand_r_sword_socket" "SnapToTarget" "SnapToTarget" "SnapToTarget" true))
    (:`else`)))

(event `Death`
  (bind _mesh (`self.Mesh`))
  ;[0.09375 0 0] Death
  ;;[0.224 0.5207 1] Detach Weapon
  (bind _weaponobject (`self.WeaponObject`)
    (:`then`
      (`/Game/Blueprints/Weapons/BP_Weapon.DetachWeapon` _weaponobject)
      (`/Game/Blueprints/Weapons/BP_Weapon.WeaponDecay` _weaponobject (`self.AfterDeathStartDecay`) (`self.DecayTime`)))
    (:`else`
      _))
  ;;[0.375 0.2908 0] Ragdoll
  (`PrimitiveComponent.SetSimulatePhysics` _mesh true)
  (`PrimitiveComponent.SetCollisionEnabled` _mesh "QueryAndPhysics")
  ;;[0 0.09948 0.1562] Remove Widget and collision
  (`ActorComponent.K2_DestroyComponent` (`self.HealthBar`))
  (`PrimitiveComponent.SetCollisionEnabled` (`self.CapsuleComponent`) "NoCollision")
  ;;[0.1875 0.1875 0.1875] Decay over time
  (`KismetSystemLibrary.Delay` (`self.AfterDeathStartDecay`))
  (`TimelineComponent.SetPlayRate` (`self.Fade`) (/ 1.0 (`self.DecayTime`)))
  (bind (_direction _fade) (`Timeline|Fade` :!via `PlayFromStart`)
    (:`Update`
      (`MaterialInstanceDynamic.SetScalarParameterValue` (`self.MeshMaterialOne`) "Fade" _fade)
      (`MaterialInstanceDynamic.SetScalarParameterValue` (`self.MeshMaterialTwo`) "Fade" _fade))
    (:`Finished`
      (`KismetSystemLibrary.Delay` 0.2)
      (`self.K2_DestroyActor`))))

(fn `CreatePatrolRoute`
  (`self.PatrolRoute`
    (:`then`)
    (:`else`
      (bind _returnvalue (`|SpawnActorFromClass` (`self.PatroulRouteClass`) (`SceneComponent.K2_GetComponentToWorld` (`self.Mesh`)) "Undefined" "MultiplyWithRoot" null null))
      (set `self.PatrolRoute` _returnvalue))))

(fn `GetCurrentHealth`
  (returns (Health :type Integer))
  (return (`/Game/Blueprints/DamageSystem/BPC_DamageSystem.Health` (`self.BPC_DamageSystem`))))

(fn `GetMaxHealth`
  (returns (MaxHealth :type Integer))
  (return (`/Game/Blueprints/DamageSystem/BPC_DamageSystem.MaxHealth` (`self.BPC_DamageSystem`))))

(fn `GetPatrolRoute`
  (returns (PatrolRoute :type "/Game/Blueprints/Enemy/AI/BP_PatrolRoute Object Reference"))
  (return (`self.PatrolRoute`)))

(fn `Heal`
  (params (Amount :type Integer))
  (returns (NewHealth :type Integer))
  (bind _newhealth (`/Game/Blueprints/DamageSystem/BPC_DamageSystem.Heal` (`self.BPC_DamageSystem`) Amount))
  (return _newhealth))

(fn `RemovePatrolRoute`
  (bind _patrolroute (`self.PatrolRoute`)
    (:`then`
      (`self.K2_DestroyActor` _patrolroute)
      (set `self.PatrolRoute` null))
    (:`else`)))

(fn `SetMovementSpeed`
  (params (Speed :type "/Game/Blueprints/Enemy/AI/Enums/E_MovementSpeed Enum" :default "NewEnumerator0"))
  (returns (SpeedValue :type "Float (double-precision)"))
  (bind _output_get (set `CharacterMovementComponent.MaxWalkSpeed` (select `/Game/Blueprints/Enemy/AI/Enums/E_MovementSpeed` Speed :`NewEnumerator1` (`self.WalkingSpeed`) :`NewEnumerator2` (`self.RunningSpeed`) :!type "Float (single-precision)") (`self.CharacterMovement`)))
  (return _output_get))

(fn `TakeDamage`
  (params (Amount :type Integer) (Location :type "Vector Structure"))
  (returns (WasDamaged :type Boolean))
  (bind _bwasdamaged (`/Game/Blueprints/DamageSystem/BPC_DamageSystem.TakeDamage` (`self.BPC_DamageSystem`) (make `/Game/Blueprints/DamageSystem/S_DamageInfo` Amount)))
  (if _bwasdamaged
    (return _bwasdamaged)))

(fn `UserConstructionScript`
  (bind _bpc_damagesystem (`self.BPC_DamageSystem`))
  (bind _output_get (set `/Game/Blueprints/DamageSystem/BPC_DamageSystem.MaxHealth` (`self.MaxHealth`) _bpc_damagesystem))
  (set `/Game/Blueprints/DamageSystem/BPC_DamageSystem.Health` _output_get _bpc_damagesystem)
  (add `/Game/Blueprints/DamageSystem/BPC_DamageSystem.OnDeath` (`self.BPC_DamageSystem`) (`|CreateDelegate` :!event `Death`))
  (bind _returnvalue (`PrimitiveComponent.CreateDynamicMaterialInstance` (`self.Mesh`) 0 (`self.SourceMaterial_01`) "None"))
  (set `self.MeshMaterialOne` _returnvalue)
  (bind _returnvalue_2 (`PrimitiveComponent.CreateDynamicMaterialInstance` (`self.Mesh`) 1 (`self.SourceMaterial_02`) "None"))
  (set `self.MeshMaterialTwo` _returnvalue_2)
  (if (`KismetSystemLibrary.IsValidClass` (`self.Weapon`))
    (set `self.bIsWieldingWeapon` true)
    (else
      (set `self.bIsWieldingWeapon` false))))