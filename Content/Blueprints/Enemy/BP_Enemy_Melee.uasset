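; BP_Enemy_Melee is a melee enemy Blueprint that extends its parent's Attack event with a sword slash.
; Attack calls the parent, then plays the slash montage at slightly reduced speed.
; Montage notify begin and end switch the weapon object's attacking state and trail on and off.
; Completion or interruption both fire OnAttackEnd, which a Behavior Tree task subscribes to.
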(event `self.Attack`
  (bind _weaponobject (`self.WeaponObject`))
  (bind _weaponobject_2 (`self.WeaponObject`))
  (`parent.Attack`)
  (bind _notifyname (`|PlayMontage` (`self.Mesh`) "/Game/Characters/Animations/Melee/AM_SwordSlash.AM_SwordSlash" 0.8)
    (:`OnCompleted`
      (`self.OnAttackEnd` :!label _label) ; Subscriber on Behavior Tree Task
    )
    (:`OnInterrupted`
      (goto _label))
    (:`OnNotifyBegin`
      (switch `name` _notifyname
        (:`Slash`
          (`/Game/Blueprints/Weapons/BP_Weapon.IsAttacking` _weaponobject true)
          (`/Game/Blueprints/Weapons/BP_Weapon.SetTrailActive` _weaponobject_2 true))))
    (:`OnNotifyEnd`
      (switch `name` _notifyname
        (:`Slash`
          (`/Game/Blueprints/Weapons/BP_Weapon.IsAttacking` _weaponobject false)
          (`/Game/Blueprints/Weapons/BP_Weapon.SetTrailActive` _weaponobject_2 false))))))

(fn `UserConstructionScript`
  (`parent.UserConstructionScript`))