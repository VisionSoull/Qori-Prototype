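; Level-placed trigger volume that puts a linked set of enemies into their attacking state when the player enters it.
; On box overlap with player pawn 0, it loops EnemiesToTrigger and calls SetStateAsAttacking on each AIC_Enemy_Base controller with the player as target.
; A CreatePassiveTrigger function spawns a PassiveStateTrigger at the same transform and hands it the same enemy list.
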(event `self.Box.OnComponentBeginOverlap`
  (params (OverlappedComponent :type "PrimitiveComponent Object Reference") (OtherActor :type "Actor Object Reference") (OtherComp :type "PrimitiveComponent Object Reference") (OtherBodyIndex :type Integer) (bFromSweep :type Boolean) (SweepResult :type "HitResult Structure (by ref)"))
  (if (== OtherActor (`GameplayStatics.GetPlayerPawn` 0))
    (for _array_element (`self.EnemiesToTrigger`)
      (bind _asaic_enemy_base (cast `/Game/Blueprints/Enemy/AI/AIC_Enemy_Base` (`AIBlueprintHelperLibrary.GetAIController` _array_element)))
      (`/Game/Blueprints/Enemy/AI/AIC_Enemy_Base.SetStateAsAttacking` _asaic_enemy_base (`GameplayStatics.GetPlayerPawn` 0)))))

(fn `CreatePassiveTrigger`
  (bind _returnvalue (`|SpawnActorFromClass` (`self.PassiveStateTrigger`) (`self.GetTransform`) "Undefined" "MultiplyWithRoot" null null))
  (set `/Game/Blueprints/Enemy/AreaTriggers/BP_Enemy_Passive_State_Trigger.EnemiesToTrigger` (`self.EnemiesToTrigger`) _returnvalue))

(fn `UserConstructionScript`)