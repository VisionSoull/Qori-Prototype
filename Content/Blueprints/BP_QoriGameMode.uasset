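; Game mode for Qori that tracks the player's checkpoint and owns the on-screen info widget.
; On begin play it clears the checkpoint and adds WBP_InfoInScreen to the viewport, with SetInfoText forwarding text to it.
; LoadCheckpoint destroys the BP_Player, then respawns it at the stored checkpoint and has that checkpoint reload its room, or reopens a level when none is valid.
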(event `self.ReceiveBeginPlay`
  (set `self.CurrentCheckpoint` null)
  (bind _returnvalue (`|CreateWidget` "/Game/UI/WBP_InfoInScreen.WBP_InfoInScreen_C" (`GameplayStatics.GetPlayerController` 0)))
  (bind _output_get (set `self.InfoInScreenWidget` _returnvalue))
  (`UserWidget.AddToViewport` _output_get 0))

(fn `LoadCheckpoint`
  (bind _asbp_player (cast `/Game/Blueprints/Player/BP_Player` (`GameplayStatics.GetPlayerCharacter` 0)))
  (`self.K2_DestroyActor` _asbp_player)
  (bind _currentcheckpoint (`self.CurrentCheckpoint`)
    (:`then`
      (`|SpawnActorFromClass` "/Game/Blueprints/Player/BP_Player.BP_Player_C" (`KismetMathLibrary.MakeTransform` (`self.K2_GetActorLocation` _currentcheckpoint)) "Undefined" "MultiplyWithRoot" null null)
      (`/Game/Blueprints/Player/BP_Checkpoint.ReloadRoom` (`self.CurrentCheckpoint`)))
    (:`else`
      (`GameplayStatics.OpenLevelBySoftObjectPtr` (`self.Level`)))))

(fn `SetInfoText`
  (params (InfoText :type Text))
  (`/Game/UI/WBP_InfoInScreen.SetInfoText` (`self.InfoInScreenWidget`) InfoText))

(fn `UpdateSpawnLocation`
  (params (CurrentCheckpoint :type "/Game/Blueprints/Player/BP_Checkpoint Object Reference"))
  (set `self.CurrentCheckpoint` CurrentCheckpoint))

(fn `UserConstructionScript`)