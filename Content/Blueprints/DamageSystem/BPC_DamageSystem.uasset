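; Damage system component that tracks health and death state for its owner.
; Heal adds health clamped between zero and MaxHealth while alive, and TakeDamage subtracts the DamageInfo amount, returning whether damage landed.
; A CanBeDamaged macro blocks damage when already dead or when the DamageInfo's DamageInvincible flag is set.
; When health reaches zero or below, it sets IsDead and fires the OnDeath dispatcher.
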(fn `Heal`
  (params (Amount :type Integer))
  (returns (NewHealth :type Integer))
  (if (not (`self.bIsDead`))
    (bind _output_get (set `self.Health` (`KismetMathLibrary.Clamp` (+ (`self.Health`) Amount) 0 (`self.MaxHealth`))))
    (return _output_get)))

(fn `TakeDamage`
  (params (DamageInfo :type "/Game/Blueprints/DamageSystem/S_DamageInfo Structure"))
  (returns (bWasDamaged :type Boolean))
  (bind (_amount _bdamageinvincible) (break `/Game/Blueprints/DamageSystem/S_DamageInfo` DamageInfo))
  (`self.CanBeDamaged` _bdamageinvincible
    (:`DoDamage`
      (bind _output_get (set `self.Health` (- (`self.Health`) _amount)))
      (if (<= _output_get 0)
        (set `self.bIsDead` true)
        (`self.OnDeath`))
      (return true))
    (:`NoDamage`
      (return false))))