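; BP_Plate is a numbered floor plate in a sequence puzzle coordinated by a PlatesManager.
; When the player pawn overlaps it while interactable, an active plate asks the manager to activate the next plate, while an inactive one resets the puzzle.
; Plate number one starts active, and state changes swap the cube's material.
; The plate also supports deactivation, disabling interaction, and removing itself from the manager before destruction.
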(event `self.Collider.OnComponentBeginOverlap`
  (params (OverlappedComponent :type "PrimitiveComponent Object Reference") (OtherActor :type "Actor Object Reference") (OtherComp :type "PrimitiveComponent Object Reference") (OtherBodyIndex :type Integer) (bFromSweep :type Boolean) (SweepResult :type "HitResult Structure (by ref)"))
  (if (== OtherActor (`GameplayStatics.GetPlayerPawn` 0))
    (if (`self.bInteractable`)
      (if (`self.bIsActive`)
        (`/Game/Blueprints/Plates/BP_PlatesManager.SetNextPlateActive` (`self.PlatesManager`) self)
        (else
          (`/Game/Blueprints/Plates/BP_PlatesManager.ResetPlates` (`self.PlatesManager`)))))))

(fn `Deactivate`
  (if (not false)
    (set `self.bIsActive` false)
    (`self.SetActiveMaterial` (`self.bIsActive`))))

(fn `DestroyPlate`
  (`/Game/Blueprints/Plates/BP_PlatesManager.RemovePlateFromArray` (`self.PlatesManager`) self)
  (`self.K2_DestroyActor`))

(fn `SetActive`
  (if (not (`self.bIsActive`))
    (set `self.bIsActive` true)
    (`self.SetActiveMaterial` (`self.bIsActive`))
    (else
      (`/Game/Blueprints/Plates/BP_PlatesManager.ResetPlates` (`self.PlatesManager`)))))

(fn `SetActiveMaterial`
  (params (bActive :type Boolean))
  ;[1 1 1] Sets the material corresponding to the plate's active state.
  (if bActive
    (`PrimitiveComponent.SetMaterial` (`self.Cube`) 0 (`self.MaterialActive`))
    (else
      (`PrimitiveComponent.SetMaterial` (`self.Cube`) 0 (`self.MaterialNormal`)))))

(fn `SetNotInteractable`
  (set `self.bInteractable` false))

(fn `SetNumber`
  (params (Number :type Integer))
  (set `self.PlateNumber` Number)
  ;[1 1 1] If the plate number is one, it means that it is the first one in the puzzle and Is Active.
  (if (== (`self.PlateNumber`) 1)
    (set `self.bIsActive` true)
    (else
      (set `self.bIsActive` false)))
  (`self.SetActiveMaterial` (`self.bIsActive`)))

(fn `SetPlatesManager`
  (params (PlatesManager :type "/Game/Blueprints/Plates/BP_PlatesManager Object Reference"))
  (set `self.PlatesManager` PlatesManager))

(fn `UserConstructionScript`)